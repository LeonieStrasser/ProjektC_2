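; BP_WeightSacrificePuzzle_Master is a puzzle that the player solves by sacrificing items until their summed weight reaches a required amount.
; It extends a parent's drop and UI events, adding each dropped item's weight, then checking completion and blocking the UI once solved.
; Every tick, an indicator lerps between min and max markers by clamped weight progress.
; Solving currently only prints a debug message.
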(event `self.ReceiveTick`
  (params (DeltaSeconds :type "Float (single-precision)"))
  (`parent.ReceiveTick` DeltaSeconds)
  (`self.UpdateWeightIndikatorPosition`))

(event `self.ReportDroppObjects`
  (params (Items :type "Array of /Game/Development/Leonie_dump/PickUps/ItemData Structure (by ref)"))
  ;[1 1 1] Player Sacrifices Objects
  (`parent.ReportDroppObjects` Items)
  (for _array_element Items
    (`self.AddItemWeight` _array_element))
  (bind _wassolved_ (`self.CheckIfPuzzleIsSolved`))
  (bind _output_get (set `self.PuzzleIsSolved` _wassolved_))
  (if _output_get
    (`self.ReportPuzzleAsSolved`)))

(event `self.OpenUIFromInput`
  ;[1 1 1] Player can Interact with Puzzle
  (if (not (`self.PuzzleIsSolved`))
    (`parent.OpenUIFromInput`)))

(event `ReportPuzzleAsSolved`
  (`KismetSystemLibrary.PrintString` "Weight Puzzle was solved!" true true (struct :`G` 1.0 :`B` 0.12875 :`A` 1.0) 5.0))

(fn `AddItemWeight`
  (params (Item :type "/Game/Development/Leonie_dump/PickUps/ItemData Structure"))
  (set `self.Sacrified_Weight` (+ (`self.Sacrified_Weight`) (`.Weight_9_EB020A074A05D53510F49D88FBD11424` (break `/Game/Development/Leonie_dump/PickUps/ItemData` Item))))
  (`KismetSystemLibrary.PrintString` (`KismetStringLibrary.Concat_StrStr` "Weight is now: " (`KismetStringLibrary.Conv_DoubleToString` (`self.Sacrified_Weight`)) " g")))

(fn `CheckIfPuzzleIsSolved`
  (returns (`WasSolved?` :type Boolean))
  (return (>= (`self.Sacrified_Weight`) (`self.MaxNeededWeight`))))

(fn `GetWeightProgress`
  (returns (CurrentWeightProgress :type "Float (double-precision)"))
  (return (`KismetMathLibrary.FClamp` (/ (`self.Sacrified_Weight`) (`self.MaxNeededWeight`)))))

(fn `UpdateWeightIndikatorPosition`
  (bind _currentweightprogress (`self.GetWeightProgress`))
  (`SceneComponent.K2_SetWorldLocation` (`self.WeightIndicator`) (`KismetMathLibrary.VLerp` (`SceneComponent.K2_GetComponentLocation` (`self.MinPosition`)) (`SceneComponent.K2_GetComponentLocation` (`self.MaxPosition`)) _currentweightprogress) false false))

(fn `UserConstructionScript`
  (`parent.UserConstructionScript`))