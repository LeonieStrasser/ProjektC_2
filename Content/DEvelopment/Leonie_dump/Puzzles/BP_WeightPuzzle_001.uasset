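; First weight riddle Blueprint in a puzzle chain, handling the puzzle's reveal and the hand-off to the next puzzle.
; PuzzleObject starts hidden, and BeginPlay prints an on-screen error if NextPuzzle is unset.
; Appear starts a Niagara effect, shows the object and uses a timeline to lerp it between two scene points.
; On solve, it calls the parent logic, stops the effect and activates NextPuzzle without a validity check.
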(event `self.ReceiveBeginPlay`
  (`parent.ReceiveBeginPlay`)
  ;[1 1 1] Visibility
  (`SceneComponent.SetVisibility` (`self.PuzzleObject`) false true)
  (`/Engine/EditorBlueprintResources/StandardMacros.IsValid` (`self.NextPuzzle`)
    (:`Is Not Valid`
      (`KismetSystemLibrary.PrintString` "Weight Riddle 001 has no Reference for Next Puzzle! LG Dr. Debug" true true (struct :`R` 1.0 :`B` 0.130888 :`A` 1.0) 20.0))))

(event `self.ReportPuzzleAsSolved`
  ;[1 1 1] Puzzle was Solved
  (`parent.ReportPuzzleAsSolved`)
  (`ActorComponent.Deactivate` (`self.Niagara_AppearEffect`))
  (`/Game/Development/Leonie_dump/Puzzles/BP_SinkableWater.Activate` (`self.NextPuzzle`)))

(event `Appear`
  ;[1 1 1] Appear Puzzle
  (`ActorComponent.Activate` (`self.Niagara_AppearEffect`) false)
  (`SceneComponent.SetVisibility` (`self.PuzzleObject`) true true)
  (bind (_direction _appearingprogress) (`Timeline|AppearingMotion` :!via `PlayFromStart`)
    (:`Update`
      (`SceneComponent.K2_SetWorldLocation` (`self.PuzzleObject`) (`KismetMathLibrary.VLerp` (`SceneComponent.K2_GetComponentLocation` (`self.StartAppearPoint`)) (`SceneComponent.K2_GetComponentLocation` (`self.EndAppearPoint`)) _appearingprogress) false false))))

(fn `UserConstructionScript`
  (`parent.UserConstructionScript`))