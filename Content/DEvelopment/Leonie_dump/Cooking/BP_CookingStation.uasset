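; Cooking station actor that combines stored consumable ingredients into a spawned food item.
; A trigger shows a widget near the player and lets the pickup input run TryMakeFood.
; TryAddIngridient accepts items of one category up to a limit; cooking needs at least two and sums their stats by type.
; SpawnFood always spawns a berry consumable, ignoring those totals; health is multiplied by zero and the list is not cleared after cooking.
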(event `self.ReceiveBeginPlay`
  (`SceneComponent.SetVisibility` (`self.Widget`) false false)
  (`self.EnableInput` (`GameplayStatics.GetPlayerController` 0)))

(event `self.Trigger.OnComponentBeginOverlap`
  (params (OverlappedComponent :type "PrimitiveComponent Object Reference") (OtherActor :type "Actor Object Reference") (OtherComp :type "PrimitiveComponent Object Reference") (OtherBodyIndex :type Integer) (bFromSweep :type Boolean) (SweepResult :type "HitResult Structure (by ref)"))
  ;[1 1 1] Range Check
  (cast `/Game/ThirdPerson/Blueprints/BP_ThirdPersonCharacter` OtherActor)
  (set `self.PlayerIsNearCooker` true)
  (`SceneComponent.SetVisibility` (`self.Widget`) true false))

(event `self.Trigger.OnComponentEndOverlap`
  (params (OverlappedComponent :type "PrimitiveComponent Object Reference") (OtherActor :type "Actor Object Reference") (OtherComp :type "PrimitiveComponent Object Reference") (OtherBodyIndex :type Integer))
  ;[1 1 1] Range Check
  (cast `/Game/ThirdPerson/Blueprints/BP_ThirdPersonCharacter` OtherActor)
  (set `self.PlayerIsNearCooker` false)
  (`SceneComponent.SetVisibility` (`self.Widget`) false false))

(event `EnhancedInput|/Game/DEvelopment/Leonie_dump/Levels_dump/IA_Pickup`
  (params (ActionValue :type Boolean) (ElapsedSeconds :type "Float (double-precision)") (TriggeredSeconds :type "Float (double-precision)") (InputAction :type "InputAction Object Reference" :default "/Game/DEvelopment/Leonie_dump/Levels_dump/IA_Pickup.IA_Pickup"))
  (:`Completed`
    (if (`self.PlayerIsNearCooker`)
      (`self.TryMakeFood`))))

(fn `ClearIngridientList`
  (`KismetArrayLibrary.Array_Clear` (`self.Ingidients`)))

(fn `SpawnFood`
  (params (NewHungerRecoverValue :type "Float (double-precision)") (NewThirstRecoverValue :type "Float (double-precision)") (NewSleepRecoverValue :type "Float (double-precision)") (NewHealthRecoverValue :type "Float (double-precision)"))
  (`|SpawnActorFromClass` "/Game/DEvelopment/Leonie_dump/PickUps/Consumabpe_Pickups/BP_Berry_Consumable.BP_Berry_Consumable_C" (`SceneComponent.K2_GetComponentToWorld` (`self.SpawnPoint`)) "Undefined" "MultiplyWithRoot" null null))

(fn `TryAddIngridient`
  (params (ConsumableItem :type "/Game/DEvelopment/Leonie_dump/PickUps/ItemData Structure"))
  (returns (`Added?` :type Boolean))
  (locals (ItemToAdd :type "/Game/DEvelopment/Leonie_dump/PickUps/ItemData Structure"))
  (bind _output_get (set `local.ItemToAdd` ConsumableItem))
  ;[1 1 1] Is Item a Consumable?
  (if (`|EnumEquality` (`.Cathegory_17_3260CCA94D6B5BA46B32838F3A435B64` (break `/Game/DEvelopment/Leonie_dump/PickUps/ItemData` _output_get)) "NewEnumerator1")
    ;[1 1 1] Is space in Ingridients List?
    (if (< (`KismetArrayLibrary.Array_Length` (`self.Ingidients`)) (`self.Ingridients_Limit`))
      ;[1 1 1] Add
      (`KismetArrayLibrary.Array_Add` (`self.Ingidients`) (`local.ItemToAdd`))
      (return true)
      (else
        (return false)))
    (else
      (return false))))

(fn `TryMakeFood`
  (returns (`MadeFood?` :type Boolean))
  (locals (HungerRecoverValue :type "Float (double-precision)") (ThirstRecoverValue :type "Float (double-precision)") (SleepRecoverValue :type "Float (double-precision)") (HealthRecoverValue :type "Float (double-precision)"))
  (if (> (`KismetArrayLibrary.Array_Length` (`self.Ingidients`)) 1)
    ;[1 1 1] ResetNewValues
    (set `local.HungerRecoverValue` 0.0)
    (set `local.ThirstRecoverValue` 0.0)
    (set `local.SleepRecoverValue` 0.0)
    (set `local.HealthRecoverValue` 0.0)
    ;[1 1 1] Create Values for new Consumable Item
    (for _array_element (`self.Ingidients`)
      (bind (_name _image _weight _description _cathegory _value _reportonpickup _timelimited _timetodistruction _amount _consumabletype _consumable_statvalue _consumable_energyvalue) (break `/Game/DEvelopment/Leonie_dump/PickUps/ItemData` _array_element))
      (switch `/Game/DEvelopment/Leonie_dump/PickUps/E_ConsumableType` _consumabletype
        (:`NewEnumerator0`
          (`KismetSystemLibrary.PrintString` "WARNING! In Try Make Food Funktion of the Cooking Station: A Consumable has arraved that has an unknown Cathegory!" true true (struct :`R` 1.0 :`G` 0.016463 :`A` 1.0) 10.0))
        (:`NewEnumerator1`
          ;;[1 1 1] Add Stat Values to a new better Value
          ;;;[1 1 1] Add Hunger Recover Value
          (set `local.HungerRecoverValue` (+ (`local.HungerRecoverValue`) _consumable_statvalue))
          ;;[1 1 1] Add Health Recover Values together
          (set `local.HealthRecoverValue` (+ (`local.HealthRecoverValue`) _consumable_energyvalue) :!label _label))
        (:`NewEnumerator2`
          ;;;[1 1 1] Add Thirst Recover Value
          (set `local.ThirstRecoverValue` (+ (`local.ThirstRecoverValue`) _consumable_statvalue))
          (goto _label))
        (:`NewEnumerator3`
          ;;;[1 1 1] Add Energy Recover Value
          (set `local.SleepRecoverValue` (+ (`local.SleepRecoverValue`) _consumable_statvalue))
          (goto _label))))
    ;;[1 1 1] Multiply Health Value (Golpalots Gesetz)
    (set `local.HealthRecoverValue` (* (`local.HealthRecoverValue`) 0.0))
    (`self.SpawnFood` (`local.HungerRecoverValue`) (`local.ThirstRecoverValue`) (`local.SleepRecoverValue`) (`local.HealthRecoverValue`))
    (return true)
    (else
      (`KismetSystemLibrary.PrintString` "Cooking Station needs min 2 Items to make food!" true true (struct :`R` 1.0 :`G` 0.788177 :`A` 1.0) 5.0)
      (return false))))

(fn `UserConstructionScript`)