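; Inventory system actor that stores picked-up items, tracks pickups in range and toggles a game-pausing inventory widget.
; Pickups enter a size-capped map as single entries keyed by name plus pickup timestamp, with add/remove events for flagged items.
; Tick counts down time-limited items and removes expired ones.
; Single or full-inventory drops respawn items at random ground points, found by retrying horizontal and downward line traces until one succeeds.
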(event `self.ReceiveBeginPlay`
  (`self.EnableInput` (`GameplayStatics.GetPlayerController` 0))
  ;[1 1 1] Set Survival Manager Reference
  (bind _outactors (`GameplayStatics.GetAllActorsOfClass` "/Game/Development/Fea_dump/BP_SurvivalManager.BP_SurvivalManager_C"))
  (set `self.Survival_Manager_ref` (`|GetArrayItem` _outactors)))

(event `self.ReceiveTick`
  (params (DeltaSeconds :type "Float (single-precision)"))
  (`self.ReduceAllLimitedLifetimesInInventory` DeltaSeconds))

(event `OpenOrCloseInventory`
  (bind _returnvalue (`GameplayStatics.GetPlayerController` 0))
  ;[1 1 1] Open and close Inventory
  (`/Engine/EditorBlueprintResources/StandardMacros.IsValid` (`self.WB_InventoryReference`)
    (:`Is Valid`
      (if (`Widget.IsVisible` (`self.WB_InventoryReference`))
        (`/Game/Development/Leonie_dump/Inventory/WBP_InventoryWidget.PlayBlenoutAnimation` (`self.WB_InventoryReference`))
        (`GameplayStatics.SetGamePaused` false)
        (`KismetSystemLibrary.Delay` 0.1)
        (`Widget.RemoveFromParent` (`self.WB_InventoryReference`))
        (`WidgetBlueprintLibrary.SetInputMode_GameOnly` _returnvalue)
        (set `PlayerController.bShowMouseCursor` false _returnvalue)
        (set `self.Inventory_is_open` false)
        (else
          (`UserWidget.AddToViewport` (stale _output_get) 0 :!label _label)
          (`WidgetBlueprintLibrary.SetInputMode_GameAndUIEx` (`GameplayStatics.GetPlayerController` 0) (`self.WB_InventoryReference`) "DoNotLock" false)
          (set `PlayerController.bShowMouseCursor` true (`GameplayStatics.GetPlayerController` 0))
          (`GameplayStatics.SetGamePaused` true)
          (set `self.Inventory_is_open` true)
          (`/Game/Development/Leonie_dump/Inventory/WBP_InventoryWidget.UpdateInventory` (`self.WB_InventoryReference`) (`self.Inventory`)))))
    (:`Is Not Valid`
      (bind _returnvalue_2 (`|CreateWidget` "/Game/Development/Leonie_dump/Inventory/WBP_InventoryWidget.WBP_InventoryWidget_C" null self))
      (bind _output_get (set `self.WB_InventoryReference` _returnvalue_2))
      (`/Engine/EditorBlueprintResources/StandardMacros.IsValid` _output_get
        (:`Is Valid`
          (goto _label))))))

(event `EnhancedInput|/Game/Development/Leonie_dump/Levels_dump/IA_Inventory`
  (params (ActionValue :type Boolean) (ElapsedSeconds :type "Float (double-precision)") (TriggeredSeconds :type "Float (double-precision)") (InputAction :type "InputAction Object Reference" :default "/Game/Development/Leonie_dump/Levels_dump/IA_Inventory.IA_Inventory"))
  ;[1 1 1] Inventory opens after Input
  (:`Completed`
    (if (not (`NavMovementComponent.IsFalling` (`Character.CharacterMovement` (`GameplayStatics.GetPlayerCharacter` 0))))
      (`self.OpenOrCloseInventory`))))

(event `ReportItemIsInRange`
  (params (NewItem :type "Actor Object Reference"))
  ;[1 1 1] Player Reports
  ;;[1 1 1] Player reports a new Item in Range
  (`self.TryPercieveItem` NewItem))

(event `LogoutItemFromRange`
  (params (Item :type "Actor Object Reference"))
  ;[1 1 1] Player Reports
  ;;[1 1 1] Player logs out an Item from Range
  (`self.TryRemoveItemFromPerceptionList` Item)
  (`KismetSystemLibrary.PrintString` "LoggedOut"))

(event `ReportDeletedItem`
  (params (ItemKey :type String) (`DropItem?` :type Boolean))
  ;[1 1 1] Delete Item
  (if `DropItem?`
    (`self.DropItem` (`BlueprintMapLibrary.Map_Find` (`self.Inventory`) ItemKey) (`SceneComponent.K2_GetComponentLocation` (`Character.Mesh` (`GameplayStatics.GetPlayerCharacter` 0)))))
  (`self.TryRemoveItem` ItemKey))

(event `ClearInventory`
  (bind _inventory (`self.Inventory`))
  ;[1 1 1] Clear Inventory
  (`BlueprintMapLibrary.Map_Clear` _inventory)
  (`/Game/Development/Leonie_dump/Inventory/WBP_InventoryWidget.UpdateInventory` (`self.WB_InventoryReference`) _inventory))

(event `DropInventoryAtPlayerLocation`
  ;[1 1 1] DroppInventory at Player Transform
  (`self.DropCompleteInventoryAtLocation` (`SceneComponent.K2_GetComponentLocation` (`Character.Mesh` (`GameplayStatics.GetPlayerCharacter` 0)))))

(fn `AddItemToInventory`
  (params (Item :type "/Game/Development/Leonie_dump/PickUps/ItemData Structure"))
  (bind (_name _image _weight _description _cathegory _value _reportonpickup _timelimited _timetodistruction _amount _consumabletype _consumable_statvalue _consumable_energyvalue _pickuptime _itemclass) (break `/Game/Development/Leonie_dump/PickUps/ItemData` Item))
  ;[1 1 1] Make sure that just one Piece of item goes to Inventory
  (bind _structout (setmembers `/Game/Development/Leonie_dump/PickUps/ItemData` :`StructRef` Item :`Amount` 1))
  (`BlueprintMapLibrary.Map_Add` (`self.Inventory`) (`KismetTextLibrary.Conv_TextToString` (`KismetTextLibrary.Conv_StringToText` (`KismetStringLibrary.Concat_StrStr` (`KismetTextLibrary.Conv_TextToString` _name) (`KismetStringLibrary.Conv_DoubleToString` _pickuptime)))) _structout)
  (if (not _timelimited)
    ;[1 1 1] Call Event for Listeners
    (if _reportonpickup
      (`self.OnItemAddedToInventory` _itemclass))))

(fn `DropCompleteInventoryAtLocation`
  (params (DropLocation :type "Vector Structure"))
  (locals (NewDropLocation :type "Vector Structure"))
  (bind _inventory (`self.Inventory`))
  (set `local.NewDropLocation` DropLocation)
  ;[1 1 1] Is something in Inventory?
  (if (> (`BlueprintMapLibrary.Map_Length` (`self.Inventory`)) 0)
    ;[1 1 1] Iterate through Inventory and drop all
    (bind _keys (`BlueprintMapLibrary.Map_Keys` _inventory))
    (for _array_element _keys
      (`self.DropItem` (`BlueprintMapLibrary.Map_Find` _inventory _array_element) (`local.NewDropLocation`)))
    (`self.ClearInventory`)
    (else
      (`KismetSystemLibrary.PrintString` "Inventory was empt. Nothing has dropped!"))))

(fn `DropItem`
  (params (Item :type "/Game/Development/Leonie_dump/PickUps/ItemData Structure") (DropCenterLocation :type "Vector Structure"))
  (bind _randomtransform (`self.GenerateRandomDropTransform` DropCenterLocation))
  (`|SpawnActorFromClass` (`.ItemClass_34_2C6ADACD4FAE8AE1A96AEBA2129A43DB` (break `/Game/Development/Leonie_dump/PickUps/ItemData` Item)) _randomtransform "Undefined" "MultiplyWithRoot" null null))

(fn `FindItemByItsKey`
  (params (Item :type "/Game/Development/Leonie_dump/PickUps/ItemData Structure"))
  (returns (ReturnValue :type Boolean))
  ;[1 1 1] Gives a bool if a item is still in the Inventory
  (return (`BlueprintMapLibrary.Map_Contains` (`self.Inventory`) (`self.MakeItemKey` Item))))

(fn `GenerateRandomDropTransform`
  (params (DropCenterLocation :type "Vector Structure"))
  (returns (RandomTransform :type "Transform Structure"))
  (locals (HasNewTransform :type Boolean) (NewTransform :type "Transform Structure"))
  (set `local.HasNewTransform` false)
  (while (== (`local.HasNewTransform`) false)
    (bind (_randomtransform _hascreatedtransform_) (`self.TryGetRandomizedDropTransform` DropCenterLocation))
    (set `local.HasNewTransform` _hascreatedtransform_)
    (if _hascreatedtransform_
      (set `local.NewTransform` _randomtransform)))
  (return (`local.NewTransform`)))

(fn `IsEnoughSpaceInInventory`
  (returns (ReturnValue :type Boolean))
  (return (< (`BlueprintMapLibrary.Map_Length` (`self.Inventory`)) (`self.AmountLimit`))))

(fn `IsTheItemAlreadyInTheInventory`
  (params (Item :type "/Game/Development/Leonie_dump/PickUps/ItemData Structure"))
  (returns (ReturnValue :type Boolean))
  ;[1 1 1] Gives a bool if a item is still in the Inventory
  (return (`BlueprintMapLibrary.Map_Contains` (`self.Inventory`) (`KismetTextLibrary.Conv_TextToString` (`.Name_4_F8E0E59F4DED3ECE3D7832A06FFC4421` (break `/Game/Development/Leonie_dump/PickUps/ItemData` Item))))))

(fn `Reduce Item Lifetime in Tick`
  (params (TimeLimitedItem :type "/Game/Development/Leonie_dump/PickUps/ItemData Structure") (DeltaSeconds :type "Float (double-precision)"))
  (returns (NewItemData :type "/Game/Development/Leonie_dump/PickUps/ItemData Structure") (`ItemwasRemoved?` :type Boolean))
  (bind ((`TimeLimited_38_90C880744F7296B737839BA816EFAF04` _timelimited) (`TimeToDistruction_41_D1C5D0634DDD1B1225FB6CBC3E58BD71` _timetodistruction)) (break `/Game/Development/Leonie_dump/PickUps/ItemData` TimeLimitedItem))
  (bind _returnvalue (`KismetMathLibrary.FClamp` (- _timetodistruction DeltaSeconds) 0.0 10000000.0))
  (if _timelimited
    (bind _structout (setmembers `/Game/Development/Leonie_dump/PickUps/ItemData` :`StructRef` TimeLimitedItem :`TimeToDistruction` _returnvalue))
    ;[1 1 1] Lösche Item wenn Zeit abgelaufen ist
    (if (== _returnvalue 0.0)
      (`self.TryRemoveItem` (`self.MakeItemKey` _structout))
      (`KismetSystemLibrary.PrintString` "Limited Lifetime Object REMOVED!!!")
      (return (struct) true)
      (else
        (return _structout false)))
    (else
      (`KismetSystemLibrary.PrintString` "Funktion \"ReduceItemLifetime\" tryed to reduce Time from an object that was not claimed as Timelimited!!! WTF!!!" true true (struct :`R` 1.0 :`B` 0.055564 :`A` 1.0) 10.0))))

(fn `ReduceAllLimitedLifetimesInInventory`
  (params (DeltaSecond :type "Float (double-precision)"))
  (bind _inventory (`self.Inventory`))
  (if (> (`BlueprintMapLibrary.Map_Length` (`self.Inventory`)) 0)
    (bind _keys (`BlueprintMapLibrary.Map_Keys` _inventory))
    (for _array_element _keys
      (bind _value (`BlueprintMapLibrary.Map_Find` _inventory _array_element))
      (if (`.TimeLimited_38_90C880744F7296B737839BA816EFAF04` (break `/Game/Development/Leonie_dump/PickUps/ItemData` _value))
        (bind (_newitemdata _itemwasremoved_) (`self.Reduce Item Lifetime in Tick` _value DeltaSecond))
        (if (not _itemwasremoved_)
          (`BlueprintMapLibrary.Map_Add` (`self.Inventory`) _array_element _newitemdata))))))

(fn `RemoveItemFromInventory`
  (params (ItemKey :type String))
  (bind _wb_inventoryreference (`self.WB_InventoryReference`))
  (bind _returnvalue (`BlueprintMapLibrary.Map_Remove` (`self.Inventory`) ItemKey))
  (if _returnvalue
    (`/Engine/EditorBlueprintResources/StandardMacros.IsValid` _wb_inventoryreference
      (:`Is Valid`
        (`/Game/Development/Leonie_dump/Inventory/WBP_InventoryWidget.UpdateInventory` _wb_inventoryreference (`self.Inventory`))))))

(fn `TimestampPickupItem`
  (params (Item :type "/Game/Development/Leonie_dump/PickUps/ItemData Structure"))
  (returns (S_ItemData :type "/Game/Development/Leonie_dump/PickUps/ItemData Structure"))
  (bind (_year _month _day _hour _minute _second _millisecond) (`KismetMathLibrary.BreakDateTime` (`KismetMathLibrary.Now`)))
  (bind _structout (setmembers `/Game/Development/Leonie_dump/PickUps/ItemData` :`StructRef` Item :`PickupTime` (`KismetStringLibrary.Conv_StringToDouble` (`KismetStringLibrary.Concat_StrStr` (`KismetStringLibrary.Conv_IntToString` _year) (`KismetStringLibrary.Conv_IntToString` _month) (`KismetStringLibrary.Conv_IntToString` _day) (`KismetStringLibrary.Conv_IntToString` _hour) (`KismetStringLibrary.Conv_IntToString` _minute) (`KismetStringLibrary.Conv_IntToString` _second) (`KismetStringLibrary.Conv_IntToString` _millisecond)))))
  (return _structout))

(fn `Try Add ItemActor`
  (params (ItemActor :type "Actor Object Reference"))
  (returns (`Added?` :type Boolean))
  ;[1 1 1] Is it a Pickup Item?
  (bind _asbp_master_pickup_item (cast `/Game/Development/Leonie_dump/PickUps/BP_MasterPickupItem` ItemActor)
    (:`then`
      (bind _output_get (set `self.currentItem` (`/Game/Development/Leonie_dump/PickUps/BP_MasterPickupItem.OverwritableItemData` _asbp_master_pickup_item)))
      (bind (_added_ _newitemdata) (`self.TryAddItem` _output_get))
      (if _added_
        (set `/Game/Development/Leonie_dump/PickUps/BP_MasterPickupItem.OverwritableItemData` _newitemdata _asbp_master_pickup_item)
        (`/Game/Development/Leonie_dump/PickUps/BP_MasterPickupItem.report_pickUp` _asbp_master_pickup_item)
        (return _added_)))
    (:`CastFailed`
      ;;[1 1 1] NEIN! Kein Pickup Item
      (set `self.currentItem` (struct)) ; Set to null if cast fails
      (`KismetSystemLibrary.PrintString` "Tried to Add an Actor to the Inventory that is not a pickup Item!" true true (struct :`R` 1.0 :`G` 0.011514 :`B` 0.141235 :`A` 1.0) 10.0)
      (return false))))

(fn `TryAddItem`
  (params (Item :type "/Game/Development/Leonie_dump/PickUps/ItemData Structure"))
  (returns (`Added?` :type Boolean) (newItemData :type "/Game/Development/Leonie_dump/PickUps/ItemData Structure"))
  (bind _returnvalue (`self.IsEnoughSpaceInInventory`))
  (if _returnvalue
    ;[1 1 1] Timestamp Pickup Item
    (bind _s_itemdata (`self.TimestampPickupItem` Item))
    (bind _output_get (set `self.currentItem` _s_itemdata))
    ;[1 1 1] Add to Inventory
    (bind _returnvalue_2 (`self.IsTheItemAlreadyInTheInventory` _output_get))
    (if _returnvalue_2
      (`KismetSystemLibrary.PrintString` "Object Stil exist in Inventory!"))
    (`self.AddItemToInventory` (`self.currentItem`))
    (return true _s_itemdata)
    (else
      (`KismetSystemLibrary.PrintString` "Inventory is full")
      (return false))))

(fn `TryGetRandomizedDropTransform`
  (params (DropCenterLocation :type "Vector Structure"))
  (returns (RandomTransform :type "Transform Structure") (`HasCreatedTransform?` :type Boolean))
  (bind (_returnvalue_x _returnvalue_y) (`KismetMathLibrary.BreakVector` (`KismetMathLibrary.RandomUnitVector`)))
  (bind _returnvalue (+ DropCenterLocation (`KismetMathLibrary.MakeVector` 0.0 0.0 50.0)))
  ;[1 1 1] Trace check horizontal
  (bind _outhit (`KismetSystemLibrary.LineTraceSingle` :`Start` _returnvalue :`End` (+ _returnvalue (* (`KismetMathLibrary.Normal` (`KismetMathLibrary.MakeVector` _returnvalue_x _returnvalue_y)) (`KismetMathLibrary.RandomFloatInRange` 10.0 200.0))) :`TraceChannel` "TraceTypeQuery1" :`DrawDebugType` "Persistent"))
  (bind (_bblockinghit _binitialoverlap _time _distance _location _impactpoint _normal _impactnormal _physmat _hitactor _hitcomponent _hitbonename _bonename _hititem _elementindex _faceindex _tracestart _traceend) (`GameplayStatics.BreakHitResult` _outhit))
  (if _bblockinghit
    (castclass `/Game/Development/Leonie_dump/PickUps/BP_MasterPickupItem` (`GameplayStatics.GetObjectClass` _hitactor)
      (:`then`
        _)
      (:`CastFailed`
        (return (struct) false))))
  ;[1 1 1] Caste nach unten zum Boden
  (bind _outhit_2 (`KismetSystemLibrary.LineTraceSingle` :`Start` _traceend :`End` (+ _traceend (0.0 0.0 -100.0)) :`TraceChannel` "TraceTypeQuery1" :`DrawDebugType` "Persistent"))
  (bind (_bblockinghit_2 _binitialoverlap_2 _time_2 _distance_2 _location_2 _impactpoint_2 _normal_2 _impactnormal_2 _physmat_2 _hitactor_2) (`GameplayStatics.BreakHitResult` _outhit_2))
  (if _bblockinghit_2
    ;;[1 1 1] Wenn die Collision ein anderes Pickup war, mach trotzdem weiter
    (castclass `/Game/Development/Leonie_dump/PickUps/BP_MasterPickupItem` (`GameplayStatics.GetObjectClass` _hitactor_2)
      (:`then`
        _)
      (:`CastFailed`
        (`KismetSystemLibrary.PrintString` "SpawnpointFound!!!!!")
        (return (`KismetMathLibrary.Conv_VectorToTransform` _location_2) true))))
  (return (struct) false))

(fn `TryPercieveItem`
  (params (ItemInRange :type "Actor Object Reference"))
  (`KismetArrayLibrary.Array_Add` (`self.PickUpsInRange`) ItemInRange)
  (`KismetSystemLibrary.PrintString` (`KismetStringLibrary.Conv_IntToString` (`KismetArrayLibrary.Array_Length` (`self.PickUpsInRange`)))))

(fn `TryRemoveItem`
  (params (ItemKey :type String))
  (bind (_value _returnvalue) (`BlueprintMapLibrary.Map_Find` (`self.Inventory`) ItemKey))
  (bind ((`ReportOnPickUp_36_8638BC7945A8A71215A187A4D1C0CD2C` _reportonpickup) (`TimeLimited_38_90C880744F7296B737839BA816EFAF04` _timelimited) (`TimeToDistruction_41_D1C5D0634DDD1B1225FB6CBC3E58BD71` _timetodistruction) (`ItemClass_34_2C6ADACD4FAE8AE1A96AEBA2129A43DB` _itemclass)) (break `/Game/Development/Leonie_dump/PickUps/ItemData` _value))
  (if _returnvalue
    (if _reportonpickup
      (`self.OnItemRemovedFromInventory` _itemclass))
    (`self.RemoveItemFromInventory` ItemKey)
    (else
      (`KismetSystemLibrary.PrintString` "Impossiple Case in BP_InventorySystem - TryRemoveItem: Couldn´t find Item in Inventory! " true true (struct :`R` 1.0 :`G` 0.040252 :`B` 0.090013 :`A` 1.0)))))

(fn `TryRemoveItemFromPerceptionList`
  (params (ItemToRemove :type "Actor Object Reference"))
  (bind _returnvalue (`KismetArrayLibrary.Array_Find` (`self.PickUpsInRange`) ItemToRemove))
  (if (>= _returnvalue 0)
    (`KismetArrayLibrary.Array_Remove` (`self.PickUpsInRange`) _returnvalue)
    (`KismetSystemLibrary.PrintString` "Item successful removed")
    (else
      (`KismetSystemLibrary.PrintString` "Item to remove not found!" true true (struct :`R` 1.0 :`B` 0.064177 :`A` 1.0) 10.0))))

(fn `UserConstructionScript`)