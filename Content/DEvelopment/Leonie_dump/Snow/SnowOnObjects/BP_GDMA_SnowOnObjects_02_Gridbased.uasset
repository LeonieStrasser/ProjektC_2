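; Generated dynamic mesh actor that builds a snow layer over chosen scene actors using Geometry Script.
; GenerateMeshCashe merges their meshes into a world-space copy and builds a BVH for downward grid raycasts.
; Hits on sufficiently upward-facing triangles spawn normal-aligned, squashable spheres.
; Optional remeshing fuses these through SDF morphology, smoothing and planar UVs, with optional tessellated texture displacement, before conversion to actor space.
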(event `ReleaseAllCompMeshes`
  (`self.ReleaseAllComputeMeshes`))

(event `GenerateMeshCashe`
  (bind _returnvalue (`GeometryScriptLibrary_MeshQueryFunctions.GetMeshBoundingBox` (`self.RecastMeshActors`)))
  (`|ExecutionSequence`
    (:`then_0`
      ;[1 1 1] Mesh initialize
      (bind _returnvalue_2 (`self.AllocateComputeMesh`))
      (set `self.RecastMeshActors` _returnvalue_2)
      (for _array_element (`self.MeshesToAddSnowTo`)
        (bind _returnvalue_3 (`self.AllocateComputeMesh`))
        (bind (_localtoworld _returnvalue_4) (`GeometryScriptLibrary_SceneUtilityFunctions.CopyMeshFromComponent` (`Actor.RootComponent` _array_element) _returnvalue_3 (struct) true null)
          (:`Failure`
            _)
          (:`Success`
            (`GeometryScriptLibrary_MeshBasicEditFunctions.AppendMesh` (`self.RecastMeshActors`) _returnvalue_4 (struct) false (struct :`CombineMode` "EnableAllMatching") null)))
        (`self.ReleaseComputeMesh` _returnvalue_3)))
    (:`then_1`
      (bind _outputbvh (`GeometryScriptLibrary_MeshSpatial.BuildBVHForMesh` (`self.RecastMeshActors`) null))
      (set `self.Output BVH` _outputbvh))
    (:`then_2`
      (if (`self.GenerateMesh`) :!label _label
        (`|ExecutionSequence`
          (:`then_0`
            ;[1 1 1] Raycast to spawn Sphere
            ;;[1 1 1] X Axis Spacing
            (for _index (range (+ (`KismetMathLibrary.Round` (/ (- (.x (`.Max` (break `Box` _returnvalue))) (.x (break `Box` _returnvalue))) (`self.GridSpacing`))) 1))
              ;;[1 1 1] Y Axis Spacing
              (for _index_2 (range (+ (`KismetMathLibrary.Round` (/ (- (.y (`.Max` (break `Box` _returnvalue))) (.y (break `Box` _returnvalue))) (`self.GridSpacing`))) 1))
                (bind _hitresult (`GeometryScriptLibrary_MeshSpatial.FindNearestRayIntersectionWithMesh` (`self.RecastMeshActors`) (`self.Output BVH`) (`KismetMathLibrary.MakeVector` (+ (.x (break `Box` _returnvalue)) (* _index (`self.GridSpacing`))) (+ (.y (break `Box` _returnvalue)) (* _index_2 (`self.GridSpacing`))) (+ (- (.z (`.Max` (break `Box` _returnvalue))) (.z (break `Box` _returnvalue))) 1000.0)) (0.0 0.0 -1.0) (struct) null)
                  (:`Found`
                    ;[1 1 1] Coverage
                    (if (`self.UseAlternatCoverageMethod`)
                      (bind (_bisvalidtriangle _returnvalue_5) (`GeometryScriptLibrary_MeshQueryFunctions.GetTriangleFaceNormal` (`self.RecastMeshActors`) (`.HitTriangleID` (break `GeometryScriptRayHitResult` _hitresult))))
                      (bind _returnvalue_6 (`KismetMathLibrary.MakeVector` (.x _returnvalue_5) (.y _returnvalue_5) (.z _returnvalue_5)))
                      ;;[1 1 1] Alternative Coverage Method
                      (if (== _returnvalue_6 (0.0 0.0 1.0) :`ErrorTolerance` (`self.SnowCoverage`))
                        (`GeometryScriptLibrary_MeshPrimitiveFunctions.AppendSphereBox` (`self.Target Mesh`) (struct) (`KismetMathLibrary.MakeTransform` (`.HitPosition` (break `GeometryScriptRayHitResult` _hitresult)) (`KismetMathLibrary.MakeRotFromZ` _returnvalue_6) (`KismetMathLibrary.MakeVector` 1.0 1.0 (`self.SnowSphereScale`))) (`self.ShpereRadius`) 6 6 6 "Center" null :!label _label_2))
                      (else
                        ;;[1 1 1] Coverage Method 1
                        (if (>= (.z _returnvalue_5) (`KismetMathLibrary.Abs` (- (`self.SnowCoverage`) 1.0)))
                          (goto _label_2)))))))))
          (:`then_1`
            ;[1 1 1] Remesh
            (if (`self.Remesh`)
              (bind _returnvalue_7 (`GeometryScriptLibrary_MeshVoxelFunctions.ApplyMeshMorphology` (`self.Target Mesh`) (make `GeometryScriptMorphologyOptions` (make `GeometryScript3DGridParameters` "GridCellSize" (`self.GridCellSize`)) false (make `GeometryScript3DGridParameters` "GridResolution") "Dilate" (`self.SnowThickness`)) null))
              (bind _returnvalue_8 (`GeometryScriptLibrary_MeshDeformFunctions.ApplyIterativeSmoothingToMesh` _returnvalue_7 (struct) (make `GeometryScriptIterativeMeshSmoothingOptions` (`self.SmoothIterations`)) null))
              (bind (_returnvalue_min _returnvalue_max) (break `Box` (`GeometryScriptLibrary_MeshQueryFunctions.GetMeshBoundingBox` _returnvalue_8)))
              (bind (_returnvalue_x _returnvalue_y) (`KismetMathLibrary.BreakVector` (- _returnvalue_max _returnvalue_min)))
              (bind _returnvalue_9 (`KismetMathLibrary.FMax` _returnvalue_x _returnvalue_y))
              (bind _returnvalue_10 (`GeometryScriptLibrary_MeshUVFunctions.SetMeshUVsFromPlanarProjection` _returnvalue_8 0 (`KismetMathLibrary.MakeTransform` (0.0 0.0 0.0) (struct) (`KismetMathLibrary.MakeVector` _returnvalue_9 _returnvalue_9 _returnvalue_9)) (struct) null))
              (bind _returnvalue_11 (`GeometryScriptLibrary_MeshNormalsFunctions.ComputeTangents` _returnvalue_10 (struct) null))
              (bind _returnvalue_12 (`GeometryScriptLibrary_MeshNormalsFunctions.ComputeSplitNormals` _returnvalue_11 (make `GeometryScriptSplitNormalsOptions` true 80.0) (struct) null))
              (bind _returnvalue_13 (`GeometryScriptLibrary_MeshUVFunctions.ScaleMeshUVs` _returnvalue_12 0 (`self.UV_Scale`) (0.5 0.5) (struct) null))
              (`GeometryScriptLibrary_MeshUVFunctions.TranslateMeshUVs` _returnvalue_13 0 (`self.UV_Offset`) (struct) null)))
          (:`then_2`
            (if (`self.Remesh`)
              (if (`self.DoMeshDisplacement`)
                (`GeometryScriptLibrary_MeshSubdivideFunctions.ApplyPNTessellation` (`self.Target Mesh`) (make `GeometryScriptPNTessellateOptions` true) (`self.SubdivisionLevel`) null)
                ;[1 1 1] Add Detail from Texture
                (bind _returnvalue_14 (`GeometryScriptLibrary_MeshDeformFunctions.ApplyDisplaceFromTextureMap` (`self.Target Mesh`) (`self.DisplacementTexture`) (struct) (make `GeometryScriptDisplaceFromTextureOptions` (`self.DisplacementAmount`) (1.0 1.0) (0.0 0.0) (`self.DisplacementCenter`) (`self.Displacement Image Channel`)) 0 null))
                (bind _returnvalue_15 (`GeometryScriptLibrary_MeshNormalsFunctions.ComputeTangents` _returnvalue_14 (struct) null))
                (`GeometryScriptLibrary_MeshNormalsFunctions.ComputeSplitNormals` _returnvalue_15 (make `GeometryScriptSplitNormalsOptions` true 90.0) (struct) null))))
          (:`then_3`
            ;[1 1 1] Correct World Position
            (`GeometryScriptLibrary_MeshTransformFunctions.TransformMesh` (`self.Target Mesh`) (`KismetMathLibrary.InvertTransform` (`self.GetTransform`)) true null)))))))

(event `self.OnRebuildGeneratedMesh`
  (params (TargetMesh :type "DynamicMesh Object Reference"))
  (set `self.Target Mesh` TargetMesh)
  (goto _label))

(fn `UserConstructionScript`)