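; Generated dynamic mesh actor that procedurally builds snow on top of selected objects using Geometry Script.
; GenerateMeshCashe merges the target actors' meshes in world space and caches a BVH for ray queries.
; Seeded random downward rays append spheres at hit points, during caching or on rebuild when GenerateMesh is set.
; The result moves to actor space, with optional morphology remeshing, smoothing, box UVs, tangents and split normals.
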(event `ReleaseAllCpmpMeshes`
  (`self.ReleaseAllComputeMeshes`))

(event `GenerateMeshCashe`
  (bind _stream (`self.Stream`))
  (bind _returnvalue (`GeometryScriptLibrary_MeshQueryFunctions.GetMeshBoundingBox` (`self.RecastMeshActors`)))
  (`|ExecutionSequence`
    (:`then_0`
      ;[1 1 1] Mesh initialize
      (bind _returnvalue_2 (`self.AllocateComputeMesh`))
      (set `self.RecastMeshActors` _returnvalue_2)
      (for _array_element (`self.MeshesToAddSnowTo`)
        (bind _returnvalue_3 (`self.AllocateComputeMesh`))
        (bind (_localtoworld _returnvalue_4) (`GeometryScriptLibrary_SceneUtilityFunctions.CopyMeshFromComponent` (`Actor.RootComponent` _array_element) _returnvalue_3 (struct) true null)
          (:`Failure`
            _)
          (:`Success`
            (`GeometryScriptLibrary_MeshBasicEditFunctions.AppendMesh` (`self.RecastMeshActors`) _returnvalue_4 (struct) false (struct :`CombineMode` "EnableAllMatching") null)))
        (`self.ReleaseComputeMesh` _returnvalue_3)))
    (:`then_1`
      (bind _outputbvh (`GeometryScriptLibrary_MeshSpatial.BuildBVHForMesh` (`self.RecastMeshActors`) null))
      (set `self.Output BVH` _outputbvh))
    (:`then_2`
      (`|ExecutionSequence` :!label _label
        (:`then_0`
          (for _ (range (+ (`self.NumberOfSpheres`) 1))
            (bind _hitresult (`GeometryScriptLibrary_MeshSpatial.FindNearestRayIntersectionWithMesh` (`self.RecastMeshActors`) (`self.Output BVH`) (`KismetMathLibrary.MakeVector` (`KismetMathLibrary.RandomFloatInRangeFromStream` _stream (.x (break `Box` _returnvalue)) (.x (`.Max` (break `Box` _returnvalue)))) (`KismetMathLibrary.RandomFloatInRangeFromStream` _stream (.y (break `Box` _returnvalue)) (.y (`.Max` (break `Box` _returnvalue)))) (+ (- (.z (`.Max` (break `Box` _returnvalue))) (.z (break `Box` _returnvalue))) 1000.0)) (0.0 0.0 -1.0) (struct) null)
              (:`Found`
                (`GeometryScriptLibrary_MeshPrimitiveFunctions.AppendSphereBox` (`self.Target Mesh`) (struct) (`KismetMathLibrary.MakeTransform` (`.HitPosition` (break `GeometryScriptRayHitResult` _hitresult))) (`self.ShpereRadius`) 6 6 6 "Center" null)))))
        (:`then_1`
          ;[1 1 1] Correct World Position
          (`GeometryScriptLibrary_MeshTransformFunctions.TransformMesh` (`self.Target Mesh`) (`KismetMathLibrary.InvertTransform` (`self.GetTransform`)) true null))
        (:`then_2`
          (if (`self.Remesh`)
            (bind _returnvalue_5 (`GeometryScriptLibrary_MeshVoxelFunctions.ApplyMeshMorphology` (`self.Target Mesh`) (make `GeometryScriptMorphologyOptions` (make `GeometryScript3DGridParameters` "GridResolution") false (make `GeometryScript3DGridParameters` "GridResolution") "Dilate" (`self.SnowThickness`)) null))
            (bind _returnvalue_6 (`GeometryScriptLibrary_MeshDeformFunctions.ApplyIterativeSmoothingToMesh` _returnvalue_5 (struct) (make `GeometryScriptIterativeMeshSmoothingOptions` (`self.SmoothIterations`)) null))
            (bind (_returnvalue_min _returnvalue_max) (break `Box` (`GeometryScriptLibrary_MeshQueryFunctions.GetMeshBoundingBox` _returnvalue_6)))
            (bind _returnvalue_7 (`GeometryScriptLibrary_MeshUVFunctions.SetMeshUVsFromBoxProjection` _returnvalue_6 0 (`KismetMathLibrary.MakeTransform` (0.0 0.0 0.0) (struct) (- _returnvalue_max _returnvalue_min)) (struct) 2 null))
            (bind _returnvalue_8 (`GeometryScriptLibrary_MeshNormalsFunctions.ComputeTangents` _returnvalue_7 (struct) null))
            (`GeometryScriptLibrary_MeshNormalsFunctions.ComputeSplitNormals` _returnvalue_8 (make `GeometryScriptSplitNormalsOptions` true 80.0) (struct) null)))))))

(event `self.OnRebuildGeneratedMesh`
  (params (TargetMesh :type "DynamicMesh Object Reference"))
  (set `self.Target Mesh` TargetMesh)
  (if (`self.GenerateMesh`)
    (goto _label)))

(fn `UserConstructionScript`)