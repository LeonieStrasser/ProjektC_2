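; Base pickup item actor that the third-person character can detect and collect.
; On BeginPlay it packs its properties into an item data struct and feeds it to a hidden WBP_PickupUI widget.
; Sphere overlaps register or remove the item with BP_ThirdPersonCharacter and toggle the widget, which turns toward the camera on Tick while in range.
; The report_pickUp event plays a sound and destroys the actor; SelfDestruct is an empty stub.
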(event `self.ReceiveBeginPlay`
  (set `self.OverwritableItemData` (make `/Game/DEvelopment/Leonie_dump/PickUps/ItemData` (`self.Name`) (`self.Image`) (`self.Weight`) (`self.Description`) (`self.Cathegory`) (`self.Value`) (`self.ReportOnPickup`) (`self.TimeLimited`) (`self.TimeToDestruction`) 1 "NewEnumerator0" 0.0 0.0 0.0 (`GameplayStatics.GetObjectClass` self)))
  ;[1 1 1] Give Widget all Item informations
  (bind _aswbp_pickup_ui (cast `/Game/DEvelopment/Leonie_dump/PickUps/WBP_PickupUI` (`WidgetComponent.GetUserWidgetObject` (`self.PickupUI`))))
  (`/Game/DEvelopment/Leonie_dump/PickUps/WBP_PickupUI.SetItemData` _aswbp_pickup_ui (`self.OverwritableItemData`))
  (`SceneComponent.SetVisibility` (`self.PickupUI`) false false))

(event `self.ReceiveTick`
  (params (DeltaSeconds :type "Float (single-precision)"))
  (if (`self.PlayerIsInRange`)
    (`self.RotateUItoPlayer`)))

(event `self.Sphere.OnComponentBeginOverlap`
  (params (OverlappedComponent :type "PrimitiveComponent Object Reference") (OtherActor :type "Actor Object Reference") (OtherComp :type "PrimitiveComponent Object Reference") (OtherBodyIndex :type Integer) (bFromSweep :type Boolean) (SweepResult :type "HitResult Structure (by ref)"))
  ;[1 1 1] Get The triggered Character
  (bind _asbp_third_person_character (cast `/Game/ThirdPerson/Blueprints/BP_ThirdPersonCharacter` OtherActor)
    (:`then`
      ;[1 1 1] Report Nex Item in Vision Cone
      (`/Game/ThirdPerson/Blueprints/BP_ThirdPersonCharacter.ReportItem` _asbp_third_person_character self)
      (`KismetSystemLibrary.PrintString` (`KismetTextLibrary.Conv_TextToString` (`self.Name`)))
      ;[1 1 1] Set UI visibility
      (set `self.PlayerIsInRange` true)
      (`SceneComponent.SetVisibility` (`self.PickupUI`) true false))
    (:`CastFailed`
      (`KismetSystemLibrary.PrintString` "Could not cast to BP_TPCharacter" true true (struct :`R` 1.0 :`B` 0.010267 :`A` 1.0) 10.0))))

(event `self.Sphere.OnComponentEndOverlap`
  (params (OverlappedComponent :type "PrimitiveComponent Object Reference") (OtherActor :type "Actor Object Reference") (OtherComp :type "PrimitiveComponent Object Reference") (OtherBodyIndex :type Integer))
  ;[1 1 1] Get The triggered Character
  (bind _asbp_third_person_character (cast `/Game/ThirdPerson/Blueprints/BP_ThirdPersonCharacter` OtherActor)
    (:`then`
      ;[1 1 1] Logout this Item from Vision Cone
      (`/Game/ThirdPerson/Blueprints/BP_ThirdPersonCharacter.LogoutItem` _asbp_third_person_character self)
      ;[1 1 1] Set UI visibility
      (set `self.PlayerIsInRange` false)
      (`SceneComponent.SetVisibility` (`self.PickupUI`) false false))
    (:`CastFailed`
      (`KismetSystemLibrary.PrintString` "Could not cast to BP_TPCharacter" true true (struct :`R` 1.0 :`B` 0.010267 :`A` 1.0) 10.0))))

(event `report_pickUp`
  (`GameplayStatics.PlaySound2D` "/Game/DEvelopment/Fea_dump/Placeholder_sounds/Items/SC_PickUp.SC_PickUp" 1.0 1.0 0.0 null null)
  (`self.K2_DestroyActor`))

(fn `RotateUItoPlayer`
  (bind _pickupui (`self.PickupUI`))
  ;[1 1 1] make UI always face the player camera
  (`SceneComponent.K2_SetWorldRotation` _pickupui (`KismetMathLibrary.FindLookAtRotation` (`SceneComponent.K2_GetComponentLocation` _pickupui) (`SceneComponent.K2_GetComponentLocation` (`PlayerCameraManager.TransformComponent` (`GameplayStatics.GetPlayerCameraManager` 0)))) false false))

(fn `SelfDestruct`)

(fn `UserConstructionScript`)