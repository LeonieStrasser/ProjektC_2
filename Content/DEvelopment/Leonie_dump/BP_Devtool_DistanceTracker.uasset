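; BP_Devtool_DistanceTracker is a debug actor that measures how far the player character moves in one second.
; Releasing the T debug key waits two seconds, then samples the character's location twice, one second apart.
; It prints the distance converted to meters as a single sample, despite the "Highest" event name.
; Separately, BeginPlay enables input and starts a one-shot delay that prints a report text after ReportTime.
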(event Custom|GetHIghestDistancePerSecond
  ;[1 1 1] Debug Get Distance Player moved in 1 second
  (CallFunction|SetStartTransform)
  (Utilities|FlowControl|Delay 1.0)
  (CallFunction|SetEndTransform)
  (bind _distance (CallFunction|GetDistance (Variables|Default|GetTransform_1) (Variables|Default|GetTransform_2)))
  (Development|PrintString (Utilities|String|Append "Player moved " (Utilities|String|ToString(Float) _distance) " m per second") true true "(R=0.000000,G=0.660000,B=1.000000,A=1.000000)" 2e+01)
  (Development|PrintString "Hello" true true "(R=0.000000,G=0.660000,B=1.000000,A=1.000000)" 2e+01))

(event Custom|ReportAfterTime
  ;[1 1 1] Timer Report
  (Utilities|FlowControl|Delay (Variables|Default|GetReportTime))
  (Development|PrintString (Utilities|String|ToString(Text) (Variables|Default|GetReportingText))))

(event EventBeginPlay
  (Input|EnableInput (Game|GetPlayerController 0))
  (CallFunction|ReportAfterTime))

(event Collision|EventActorBeginOverlap
  (params (OtherActor :type Actor%20Object%20Reference)))

(event EventTick
  (params (DeltaSeconds :type Float%20%28single-precision%29)))

(event Input|KeyboardEvents|DebugKeyT
  (params (Key :type Key%20Structure) (ActionValue :type Input%20Action%20Value%20Structure))
  ;[1 1 1] Debug Get Distance Player moved in 1 second
  (:Released
    (Utilities|FlowControl|Delay 2.0)
    (CallFunction|GetHIghestDistancePerSecond)))

(fn ConstructionScript)

(fn SetStartTransform
  (Variables|Default|SetTransform_1 (Transformation|GetActorLocation (Game|GetPlayerCharacter 0))))

(fn SetEndTransform
  (Variables|Default|SetTransform_2 (Transformation|GetActorLocation (Game|GetPlayerCharacter 0))))

(fn GetDistance
  (params (Transform_1 :type Vector) (Transform_2 :type Vector))
  (return (/ (Math|Vector|Distance(Vector) Transform_1 Transform_2) 1e+02)))