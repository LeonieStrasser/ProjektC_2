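; BP_Bed is a bed actor that shows a floating UI widget while the third-person player is inside its collision.
; On overlap it looks up an item in the inventory to choose the upgrade or standard bed widget, and flags player proximity and upgrade ownership.
; Tick billboards the widget toward the camera, and ResetUI restores the standard widget.
; BeginPlay sets InventoryRef to None, so its validity check always logs a missing inventory.
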(event OnComponentBeginOverlap(collision)
  (params (OverlappedComponent :type Primitive%20Component%20Object%20Reference) (OtherActor :type Actor%20Object%20Reference) (OtherComp :type Primitive%20Component%20Object%20Reference) (OtherBodyIndex :type Integer) (bFromSweep :type Boolean) (SweepResult :type Hit%20Result%20Structure%20%28by%20ref%29))
  (Utilities|Casting|CastToBP_ThirdPersonCharacter OtherActor)
  (Variables|Default|SetPlayer_is_near_bed true)
  (if true
    (bind _returnvalue (CallFunction|FindItembyItsKey (.Inventory_ref (Variables|Default|GetInventory_ref))))
    (if _returnvalue
      (bind _returnvalue_2 (UserInterface|CreateWidget "/Game/DEvelopment/Fea_dump/UI/WB_Bed_UI_upgrade.WB_Bed_UI_upgrade_C" (Game|GetPlayerController 0)))
      (UserInterface|SetWidget (Variables|Default|GetUI) _returnvalue_2)
      (Variables|Default|SetPlayer_has_BedUpgrade true)
      (else
        (UserInterface|SetWidget (Variables|Default|GetUI) (stale _returnvalue))))
    (Rendering|SetVisibility (Variables|Default|GetUI) true false)))

(event OnComponentEndOverlap(collision)
  (params (OverlappedComponent :type Primitive%20Component%20Object%20Reference) (OtherActor :type Actor%20Object%20Reference) (OtherComp :type Primitive%20Component%20Object%20Reference) (OtherBodyIndex :type Integer))
  (Utilities|Casting|CastToBP_ThirdPersonCharacter)
  (Variables|Default|SetPlayer_is_near_bed false)
  (Rendering|SetVisibility (Variables|Default|GetUI) false false))

(event Custom|ResetUI
  (bind _returnvalue (UserInterface|CreateWidget "/Game/DEvelopment/Fea_dump/UI/WB_Bed_UI.WB_Bed_UI_C" (Game|GetPlayerController 0)))
  (UserInterface|SetWidget (Variables|Default|GetUI) _returnvalue))

(event EventBeginPlay
  (bind _outactors (Actor|GetAllActorsOfClass 0))
  (bind _output_get (Variables|Default|SetInventory_ref 0 0))
  (Utilities|IsValid _output_get
    (:Is%20Valid
      (bind _outactors_2 (Actor|GetAllActorsOfClass 0))
      (Utilities|IsValid (Utilities|Array|Get(acopy) _outactors_2)
        (:Is%20Not%20Valid
          (Development|PrintString "BP_Bed can not find an BP_BedUpgrade in Scene" true true "(R=1.000000,G=0.000000,B=0.007701,A=1.000000)" 2e+01))))
    (:Is%20Not%20Valid
      (Development|PrintString "BP_Bed can not find an BP_Inventory_System in Scene" true true "(R=1.000000,G=0.000000,B=0.026767,A=1.000000)" 2e+01))))

(event EventTick
  (params (DeltaSeconds :type Float%20%28single-precision%29))
  (bind _ui (Variables|Default|GetUI))
  ;[1 1 1] make UI always face the player camera
  (Transformation|SetWorldRotation _ui (Math|Rotator|FindLookatRotation (Transformation|GetWorldLocation _ui) (Transformation|GetWorldLocation (Variables|/Script/Engine.PlayerCameraManager|GetTransformComponent (Game|GetPlayerCameraManager 0)))) false false))

(fn ConstructionScript)