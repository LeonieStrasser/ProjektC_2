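; BP_Bed_Upgrade is a pickup item that passes upgrade data to the bed actor.
; On BeginPlay it caches the first BP_Bed found in the level through GetAllActorsOfClass.
; When pickup is reported, it writes its OverwritableItemData into that bed's UpgradeData, then runs the parent's pickup logic.
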(event `self.report_pickUp`
  (set `/Game/DEvelopment/Fea_dump/BP_Bed.Upgrade_data` (`self.OverwritableItemData`) (`self.Bed_ref`))
  (`parent.report_pickUp`))

(event `self.ReceiveBeginPlay`
  (`parent.ReceiveBeginPlay`)
  (bind _outactors (`GameplayStatics.GetAllActorsOfClass` "/Game/DEvelopment/Fea_dump/BP_Bed.BP_Bed_C"))
  (set `self.Bed_ref` (`|GetArrayItem` _outactors)))

(fn `UserConstructionScript`
  (`parent.UserConstructionScript`))