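; Base area spawner that scatters a random number of actors of a configurable class inside its SpawnArea bounds and refreshes them each night.
; Tick spawns one actor per frame at a random point until the count, rolled between min and max, is reached.
; When BP_SurvivalManager reports night, a DoOnce gate destroys the tracked actors and rerolls the count, triggering a respawn; the gate rearms during the day.
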(event `self.ReceiveBeginPlay`
  (bind _outactors (`GameplayStatics.GetAllActorsOfClass` "/Game/Development/Fea_dump/BP_SurvivalManager.BP_SurvivalManager_C"))
  (set `self.survival_manager_ref` (`|GetArrayItem` _outactors))
  ;[1 1 1] initial set up for spawning
  (set `self.Items_spawned` 0)
  (set `self.Items_to_be_spawned` (`KismetMathLibrary.RandomIntegerInRange` (`self.Min_spawn_amount`) (`self.Max_spawn_amount`)))
  (`KismetArrayLibrary.Array_Clear` (`self.spawned_actors_array`)))

(event `self.ReceiveTick`
  (params (DeltaSeconds :type "Float (single-precision)"))
  (if (== (`self.Items_spawned`) (`self.Items_to_be_spawned`))
    (if (`/Game/Development/Fea_dump/BP_SurvivalManager.At_night` (`self.survival_manager_ref`))
      (`/Engine/EditorBlueprintResources/StandardMacros.DoOnce` false :!label _label
        (:`Completed`
          (`self.Reset`)))
      (else
        (goto _label :!via `Reset`)))
    (else
      (`self.Spawn_inArea`))))

(event `Spawn_inArea`
  (bind (_origin _boxextent) (`KismetSystemLibrary.GetComponentBounds` (`self.spawn_area`)))
  ;[1 1 1] spawning
  (`|SpawnActorFromClass` (`self.SpawnItem_Class`) (`KismetMathLibrary.MakeTransform` (`KismetMathLibrary.RandomPointInBoundingBox` _origin _boxextent)) "Undefined" "MultiplyWithRoot" null null)
  (set `self.Items_spawned` (+ (`self.Items_spawned`) 1))
  (`KismetArrayLibrary.Array_Add` (`self.spawned_actors_array`)))

(event `Reset`
  (bind _spawned_actors_array (`self.spawned_actors_array`))
  ;[1 1 1] remove all previously spawned items
  (for _index (range (+ (`KismetArrayLibrary.Array_Length` _spawned_actors_array) 1))
    (`self.K2_DestroyActor` (`|GetArrayItem` _spawned_actors_array _index)))
  ;[1 1 1] reset parameters for spawning
  (set `self.Items_spawned` 0)
  (set `self.Items_to_be_spawned` (`KismetMathLibrary.RandomIntegerInRange` (`self.Min_spawn_amount`) (`self.Max_spawn_amount`)))
  (`KismetArrayLibrary.Array_Clear` (`self.spawned_actors_array`)))

(fn `UserConstructionScript`)