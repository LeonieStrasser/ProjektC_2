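; BP_Base is the player's base actor, which tracks whether the player is inside it and respawns them there after a game over.
; Box overlap begin and end events set PlayerIsAtBase for BP_ThirdPersonCharacter.
; SpawnPlayerAfterGameOver waits briefly, then teleports player 0's existing character to a random point within the RespawnArea bounds and prints a message.
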(event `self.Box.OnComponentBeginOverlap`
  (params (OverlappedComponent :type "PrimitiveComponent Object Reference") (OtherActor :type "Actor Object Reference") (OtherComp :type "PrimitiveComponent Object Reference") (OtherBodyIndex :type Integer) (bFromSweep :type Boolean) (SweepResult :type "HitResult Structure (by ref)"))
  (cast `/Game/ThirdPerson/Blueprints/BP_ThirdPersonCharacter` OtherActor)
  (set `self.Player_is_at_base` true))

(event `SpawnPlayerAfterGameOver`
  (bind (_origin _boxextent) (`KismetSystemLibrary.GetComponentBounds` (`self.respawn_area`)))
  (`KismetSystemLibrary.Delay` 0.4)
  (`self.K2_SetActorTransform` (`GameplayStatics.GetPlayerCharacter` 0) (`KismetMathLibrary.MakeTransform` (`KismetMathLibrary.RandomPointInBoundingBox` _origin _boxextent)) false true)
  (`KismetSystemLibrary.PrintString` "Respawned"))

(event `self.Box.OnComponentEndOverlap`
  (params (OverlappedComponent :type "PrimitiveComponent Object Reference") (OtherActor :type "Actor Object Reference") (OtherComp :type "PrimitiveComponent Object Reference") (OtherBodyIndex :type Integer))
  (cast `/Game/ThirdPerson/Blueprints/BP_ThirdPersonCharacter` OtherActor)
  (set `self.Player_is_at_base` false))

(fn `UserConstructionScript`)