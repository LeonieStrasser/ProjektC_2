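; Survival manager actor that tracks the player's Food, Drink, Sleep and Energy and creates a widget on start.
; Tick drains the needs; empty needs and cold or night away from BP_Base add debuffs that drain Energy.
; At zero Energy it flags GameOver and refills stats to fractions of max; its fade sequence is unwired.
; Events restore stats, report cold and handle waking; Eating ignores its inputs for fixed gains.
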(event `self.ReceiveBeginPlay`
  (bind _food_drink_sleep_maxvalue (`self.Food_Drink_Sleep_MaxValue`))
  (bind _outactors (`GameplayStatics.GetAllActorsOfClass` null))
  (set `self.Inventory_system_ref` null)
  (bind _outactors_2 (`GameplayStatics.GetAllActorsOfClass` "/Game/DEvelopment/Blueprints/Actors/BP_Base.BP_Base_C"))
  (set `self.Base_ref` (`|GetArrayItem` _outactors_2))
  (`|ExecutionSequence`
    (:`then_0`
      ;[1 1 1] initial set (default values)
      (set `self.Energy` (`self.Energy_maxValue`))
      (set `self.Food` _food_drink_sleep_maxvalue)
      (set `self.Drink` _food_drink_sleep_maxvalue)
      (set `self.Sleep` _food_drink_sleep_maxvalue))
    (:`then_1`
      (bind _returnvalue (`|CreateWidget` null))
      (`UserWidget.AddToViewport` _returnvalue 0))))

(event `self.ReceiveTick`
  (params (DeltaSeconds :type "Float (single-precision)"))
  (bind _returnvalue (/ (`self.Food_Drink_Sleep_MaxValue`) (`self.GameOver_divider_stats`)))
  (bind _player_is_at_base (`/Game/DEvelopment/Blueprints/Actors/BP_Base.Player_is_at_base` (`self.Base_ref`)))
  ;[1 1 1] values for food , sleep and drink go down constantly
  (set `self.Food` (- (`self.Food`) (* DeltaSeconds (`self.Food_loss_multiplier`))))
  (set `self.Drink` (- (`self.Drink`) (* DeltaSeconds (`self.Drink_loss_multiplier`))))
  (set `self.Sleep` (- (`self.Sleep`) (* DeltaSeconds (`self.Sleep_loss_multiplier`))))
  (`|ExecutionSequence`
    (:`then_0`
      ;[1 1 1] check for debuffs
      (if (<= (`self.Food`) 0.0)
        (set `self.PlayerIsHungry` true)
        (set `self.Food` 0.0)
        ;[1 1 1] add debuff
        (`/Engine/EditorBlueprintResources/StandardMacros.DoOnce` false :!label _label
          (:`Completed`
            (set `self.debuff_multiplier_hungry` (+ (`self.debuff_multiplier_hungry`) (`self.debuff_hunger_amount`)))
            (goto _label_2 :!via `Reset`)))
        (else
          (set `self.PlayerIsHungry` false)
          ;[1 1 1] remove debuff if resource gets filled again
          (if (not (== (`self.debuff_multiplier_hungry`) 0.0))
            (`/Engine/EditorBlueprintResources/StandardMacros.DoOnce` false :!label _label_2
              (:`Completed`
                (set `self.debuff_multiplier_hungry` (- (`self.debuff_multiplier_hungry`) (`self.debuff_hunger_amount`)))
                (goto _label :!via `Reset`)))))))
    (:`then_1`
      (if (<= (`self.Drink`) 0.0)
        (set `self.PlayerIsThirsty` true)
        (set `self.Drink` 0.0)
        (`/Engine/EditorBlueprintResources/StandardMacros.DoOnce` false :!label _label_3
          (:`Completed`
            (set `self.debuff_multiplier_thirsty` (+ (`self.debuff_multiplier_thirsty`) (`self.debuff_thirst_amount`)))
            (goto _label_4 :!via `Reset`)))
        (else
          (set `self.PlayerIsThirsty` false)
          (if (not (== (`self.debuff_multiplier_thirsty`) 0.0))
            (`/Engine/EditorBlueprintResources/StandardMacros.DoOnce` false :!label _label_4
              (:`Completed`
                (set `self.debuff_multiplier_thirsty` (- (`self.debuff_multiplier_thirsty`) (`self.debuff_thirst_amount`)))
                (goto _label_3 :!via `Reset`)))))))
    (:`then_2`
      (if (<= (`self.Sleep`) 0.0)
        (set `self.PlayerIsTired` true)
        (set `self.Sleep` 0.0)
        (`/Engine/EditorBlueprintResources/StandardMacros.DoOnce` false :!label _label_5
          (:`Completed`
            (set `self.debuff_multiplier_tired` (+ (`self.debuff_multiplier_tired`) (`self.debuff_tired_amount`)))
            (goto _label_6 :!via `Reset`)))
        (else
          (set `self.PlayerIsTired` false)
          (if (not (== (`self.debuff_multiplier_tired`) 0.0))
            (`/Engine/EditorBlueprintResources/StandardMacros.DoOnce` false :!label _label_6
              (:`Completed`
                (set `self.debuff_multiplier_tired` (- (`self.debuff_multiplier_tired`) (`self.debuff_tired_amount`)))
                (goto _label_5 :!via `Reset`)))))))
    (:`then_3`
      (if (`self.Player_is_cold`)
        (set `self.debuff_multiplier_night` (`self.debuff_night_amount`) :!label _label_7)
        (set `self.player_gets_frost_damage` true)))
    (:`then_4`
      (if (and (not _player_is_at_base) (`self.At_night`))
        (goto _label_7)))
    (:`then_5`
      (if (not (or (`self.Player_is_cold`) (`self.At_night`)))
        (set `self.debuff_multiplier_night` 0.0 :!label _label_8)
        (set `self.player_gets_frost_damage` false)))
    (:`then_6`
      (if _player_is_at_base
        (goto _label_8)))
    (:`then_7`
      ;[1 1 1] manage energy
      (set `self.Energy` (- (`self.Energy`) (* DeltaSeconds (+ (`self.debuff_multiplier_hungry`) (`self.debuff_multiplier_thirsty`) (`self.debuff_multiplier_tired`) (`self.debuff_multiplier_night`)))))
      ;[1 1 1] game Over
      (if (<= (`self.Energy`) 0.0)
        (set `self.GameOver` true)
        (`/Engine/EditorBlueprintResources/StandardMacros.DoOnce` false :!label _label_9
          (:`Completed`
            (set `self.Food` _returnvalue)
            (set `self.Sleep` _returnvalue)
            (set `self.Drink` _returnvalue)
            (set `self.Energy` (/ (`self.Energy_maxValue`) (`self.GameOver_divider_Energy`)))))
        (else
          (set `self.GameOver` false)
          (goto _label_9 :!via `Reset`))))))

(event `Eating`
  (params (Food_Gain_Value :type "Float (double-precision)") (Energy_Gain_Value :type "Float (double-precision)"))
  (bind _energy_maxvalue (`self.Energy_maxValue`))
  (bind _food_drink_sleep_maxvalue (`self.Food_Drink_Sleep_MaxValue`))
  ;[1 1 1] Events to gain Ressources
  (set `self.Food` (+ (`self.Food`) 10.0))
  (set `self.Energy` (+ (`self.Energy`) 10.0))
  (if (>= (`self.Energy`) _energy_maxvalue)
    (set `self.Energy` _energy_maxvalue))
  (if (>= (`self.Food`) _food_drink_sleep_maxvalue)
    (set `self.Food` _food_drink_sleep_maxvalue)))

(event `Reset_after_sleeping`
  ;[1 1 1] Reset After Sleeping
  (bind _outactor (`LevelSequencePlayer.CreateLevelSequencePlayer` null))
  (`MovieSceneSequencePlayer.Play` (`LevelSequenceActor.SequencePlayer` _outactor))
  (set `self.Player_just_slept` true)
  (`KismetSystemLibrary.Delay` 1.0)
  (set `self.Player_just_slept` false))

(event `Sleeping`
  (params (Sleep_Gain_Value :type "Float (double-precision)") (Energy_Gain_Value :type "Float (double-precision)"))
  (bind _energy_maxvalue (`self.Energy_maxValue`))
  (bind _food_drink_sleep_maxvalue (`self.Food_Drink_Sleep_MaxValue`))
  ;[1 1 1] Events to gain Ressources
  (set `self.Sleep` (+ (`self.Sleep`) Sleep_Gain_Value))
  (set `self.Energy` (+ (`self.Energy`) Energy_Gain_Value))
  (if (>= (`self.Energy`) _energy_maxvalue)
    (set `self.Energy` _energy_maxvalue))
  (if (>= (`self.Sleep`) _food_drink_sleep_maxvalue)
    (set `self.Sleep` _food_drink_sleep_maxvalue)))

(event `Report_Coldness`
  (set `self.Player_is_cold` true))

(event `Report_noMoreColdness`
  (set `self.Player_is_cold` false))

(event `Drinking`
  (params (Drink_Gain_Value :type "Float (double-precision)") (Energy_Gain_Value :type "Float (double-precision)"))
  (bind _energy_maxvalue (`self.Energy_maxValue`))
  (bind _food_drink_sleep_maxvalue (`self.Food_Drink_Sleep_MaxValue`))
  ;[1 1 1] Events to gain Ressources
  (set `self.Drink` (+ (`self.Drink`) Drink_Gain_Value))
  (set `self.Energy` (+ (`self.Energy`) Energy_Gain_Value))
  (if (>= (`self.Energy`) _energy_maxvalue)
    (set `self.Energy` _energy_maxvalue))
  (if (>= (`self.Drink`) _food_drink_sleep_maxvalue)
    (set `self.Drink` _food_drink_sleep_maxvalue)))

(fn `UserConstructionScript`)